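; BP_HeroChar is the player hero character, handling movement, look, jump, sprint and gun firing input.
; On BeginPlay it applies the walk speed, then spawns a BP_SKGun and attaches it to the right-hand socket of the Arms component.
; Sprint swaps the movement component's max speed while held, and fire forwards trigger press and release to the stored gun reference.
; Both inputs also set IsSprinting and IsFiring state flags.
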(event `self.ReceiveBeginPlay`
  (`|ExecutionSequence`
    (:`then_0`
      ;[1 1 1] Set Max Walk Speed
      (set `CharacterMovementComponent.MaxWalkSpeed` (`self.WalkSpeed`) (`self.CharacterMovement`)))
    (:`then_1`
      ;[1 1 1] Gun Spawn
      (bind _returnvalue (`|SpawnActorFromClass` "/Game/HeroChar/Gun/SKGun/BP_SKGun.BP_SKGun_C" (`self.Spawn Arma`) "Undefined" "OverrideRootScale" null null))
      (bind _output_get (set `self.BPGunRefer` _returnvalue))
      (`self.K2_AttachToComponent` _output_get (`self.Arms`) "hand_rSocket" "KeepRelative" "KeepRelative" "KeepRelative" false))))

(event `InputAxis|MoveForward`
  (params (AxisValue :type "Float (single-precision)"))
  ;[1 1 1] Movimento Basico
  (`self.AddMovementInput` (`SceneComponent.GetForwardVector` (`self.CapsuleComponent`)) AxisValue))

(event `InputAction|JumpButton`
  (params (Key :type "Key Structure"))
  ;[1 1 1] Pulo
  (:`Pressed`
    (`self.Jump`))
  (:`Released`
    (`self.StopJumping`)))

(event `InputAxis|MoveRight`
  (params (AxisValue :type "Float (single-precision)"))
  ;[1 1 1] Movimento Basico
  (`self.AddMovementInput` (`SceneComponent.GetRightVector` (`self.CapsuleComponent`)) AxisValue))

(event `InputAction|SprintButton`
  (params (Key :type "Key Structure"))
  (bind _charactermovement (`self.CharacterMovement`))
  ;[1 1 1] Sprint
  (:`Pressed`
    (set `self.isSprinting` true)
    (set `CharacterMovementComponent.MaxWalkSpeed` (`self.SprintSpeed`) _charactermovement))
  (:`Released`
    (set `self.isSprinting` false)
    (set `CharacterMovementComponent.MaxWalkSpeed` (`self.WalkSpeed`) _charactermovement)))

(event `InputAxis|LookTurn`
  (params (AxisValue :type "Float (single-precision)"))
  ;[1 1 1] Movimento Basico
  (`self.AddControllerYawInput` AxisValue))

(event `InputAxis|LookUp`
  (params (AxisValue :type "Float (single-precision)"))
  ;[1 1 1] Movimento Basico
  (`self.AddControllerPitchInput` AxisValue))

(event `InputAction|FireButton`
  (params (Key :type "Key Structure"))
  (bind _bpgunrefer (`self.BPGunRefer`))
  ;[1 1 1] Fire
  (:`Pressed`
    (`/Game/HeroChar/Gun/SKGun/BP_SKGun.Active Trigger` _bpgunrefer)
    (set `self.isFiring` true))
  (:`Released`
    (`/Game/HeroChar/Gun/SKGun/BP_SKGun.Deactive Trigger` _bpgunrefer)
    (set `self.isFiring` false)))

(fn `UserConstructionScript`)